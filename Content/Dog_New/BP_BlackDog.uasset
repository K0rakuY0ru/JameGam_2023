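; BP_BlackDog is a dog enemy that chases the player and can be killed with a hammer.
; PawnSensing sets a seen flag and triggers an AI MoveTo toward the seen BP_TopDown_Char.
; Capsule overlaps with a Hammer subtract its damage from Life, gated by a DoOnce that resets after a short delay, and destroy the dog at zero or below.
; A TextRender displays current Life, refreshed every Tick.
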(event `self.CapsuleComponent.OnComponentBeginOverlap`
  (params (OverlappedComponent :type "PrimitiveComponent Object Reference") (OtherActor :type "Actor Object Reference") (OtherComp :type "PrimitiveComponent Object Reference") (OtherBodyIndex :type Integer) (bFromSweep :type Boolean) (SweepResult :type "HitResult Structure (by ref)"))
  (bind _ashammer (cast `/Game/Character/Hammer/Hammer` OtherActor))
  (`/Engine/EditorBlueprintResources/StandardMacros.DoOnce` false :!label _label
    (:`Completed`
      (bind _output_get (set `self.Life` (- (`self.Life`) (`/Game/Character/Hammer/Hammer.HammerDMG` _ashammer))))
      (if (<= _output_get 0)
        (`self.K2_DestroyActor`)
        (else
          (`KismetSystemLibrary.Delay` 0.7)
          (goto _label :!via `Reset`))))))

(event `self.ReceiveTick`
  (params (DeltaSeconds :type "Float (single-precision)"))
  (`TextRenderComponent.K2_SetText` (`self.TextRender`) (`KismetTextLibrary.Conv_IntToText` (`self.Life`))))

(event `self.PawnSensing.OnSeePawn`
  (params (Pawn :type "Pawn Object Reference"))
  (set `self.isSeengPlayer` true)
  (`self.FollowPlayer`))

(event `FollowPlayer`
  (if (`self.isSeengPlayer`)
    (bind _asbp_top_down_char (cast `/Game/Character/BP_TopDown_Char` (stale `self.PawnSensing.OnSeePawn` Pawn)))
    (`|AIMoveTo` self (0.0 0.0 0.0) _asbp_top_down_char)))

(fn `UserConstructionScript`)